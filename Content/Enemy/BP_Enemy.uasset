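; BP_Enemy is an enemy that roams the level, chases the player and triggers game over on contact.
; It patrols by repeatedly moving to random reachable points around itself with AI MoveTo.
; Pawn sensing or a sound trigger overlap switches it to chasing, and it resumes roaming after a retriggerable delay or when the player leaves the sound trigger.
; A death trigger overlap with the player calls GameOver on the Manager actor.
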(event `self.ReceiveBeginPlay`
  ;[0 0 0] Patrol, move enemy to a random point
  (`self.Random Roam`))

(event `self.PawnSensing.OnSeePawn`
  (params (Pawn :type "Pawn Object Reference"))
  ;[0 0 0] See Player
  (`|ExecutionSequence`
    (:`then_0`
      (`|AIMoveTo` self (0.0 0.0 0.0) Pawn))
    (:`then_1`
      (`KismetSystemLibrary.RetriggerableDelay` 3.0)
      (`self.Random Roam`))))

(event `Random Roam`
  ;[0 0 0] Patrol, move enemy to a random point
  (`|AIMoveTo` self (`NavigationSystemV1.K2_GetRandomReachablePointInRadius` (`self.K2_GetActorLocation`) 2500.0 null null) null
    (:`OnSuccess`
      (`self.Random Roam`))))

(event `self.soundtrigger.OnComponentBeginOverlap`
  (params (OverlappedComponent :type "PrimitiveComponent Object Reference") (OtherActor :type "Actor Object Reference") (OtherComp :type "PrimitiveComponent Object Reference") (OtherBodyIndex :type Integer) (bFromSweep :type Boolean) (SweepResult :type "HitResult Structure (by ref)"))
  ;[0 0 0] Hear Player
  (bind _asbp_first_person_character (cast `/Game/FirstPerson/Blueprints/BP_FirstPersonCharacter` OtherActor))
  (`|AIMoveTo` self (0.0 0.0 0.0) _asbp_first_person_character))

(event `self.dedtrigger.OnComponentBeginOverlap`
  (params (OverlappedComponent :type "PrimitiveComponent Object Reference") (OtherActor :type "Actor Object Reference") (OtherComp :type "PrimitiveComponent Object Reference") (OtherBodyIndex :type Integer) (bFromSweep :type Boolean) (SweepResult :type "HitResult Structure (by ref)"))
  ;[0 0 0] Kill Player
  (cast `/Game/FirstPerson/Blueprints/BP_FirstPersonCharacter` OtherActor)
  (set `self.IsPlayerDed` true)
  (bind _returnvalue (`GameplayStatics.GetActorOfClass` "/Game/Blueprints/Manager.Manager_C"))
  (`/Game/Blueprints/Manager.GameOver` _returnvalue))

(event `self.soundtrigger.OnComponentEndOverlap`
  (params (OverlappedComponent :type "PrimitiveComponent Object Reference") (OtherActor :type "Actor Object Reference") (OtherComp :type "PrimitiveComponent Object Reference") (OtherBodyIndex :type Integer))
  ;[0 0 0] Hear Player
  (cast `/Game/FirstPerson/Blueprints/BP_FirstPersonCharacter` OtherActor)
  (`self.Random Roam`))

(fn `UserConstructionScript`)